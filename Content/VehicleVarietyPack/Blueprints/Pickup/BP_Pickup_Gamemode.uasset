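; BP_Pickup_Gamemode is the game mode for the pickup vehicle, handling HUD setup and a countdown.
; BeginPlay creates the HUD and timer widgets and adds both to the viewport.
; Tick runs the countdown through a one-second Delay, lowering Seconds by one after each wait while it is above zero.
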(event EventBeginPlay
  ;[1 1 1] HUDWidget
  (bind _returnvalue (UserInterface|CreateWidget "/Game/Blueprints/BP_HUDWidget.BP_HUDWidget_C"))
  (UserInterface|Viewport|AddtoViewport _returnvalue 0)
  (bind _returnvalue_2 (UserInterface|CreateWidget "/Game/Blueprints/BP_TimerWidget.BP_TimerWidget_C"))
  (UserInterface|Viewport|AddtoViewport _returnvalue_2 0))

(event EventTick
  (params (DeltaSeconds :type Float%20%28single-precision%29))
  ;[1 1 1] WaitForStart
  (if (> (Variables|Default|GetSeconds) 0)
    (Utilities|FlowControl|Delay 1.0)
    (Variables|Default|SetSeconds (- (Variables|Default|GetSeconds) 1))))

(fn ConstructionScript)